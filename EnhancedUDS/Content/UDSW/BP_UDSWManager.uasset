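; Manager that drives Ultra Dynamic Sky and Weather from tagged BP_UDSWConfig entries, using externally supplied actor references.
; Each tag applies sky and weather presets, time of day (instant on first use), sky modifier swaps with fades, and a weather change.
; Separate preset functions, disconnected in the event graph, copy values by property name and type, skipping sky properties that weather overwrites.
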(event `self.ClearAndApplyUDSWCfgEntry`
  (params (Tag :type "GameplayTag Structure"))
  (bind _uds (`self.UDS`))
  (bind _lastudsmodifiers (`self.LastUDSModifiers`))
  (`self.UDS`
    (:`then`
      (`self.UDW`
        (:`then`
          (bind _returnvalue (`self.GetUDSWCfg`))
          (bind _asbp_udswconfig (cast `/Game/UltraDynamicSky/Blueprints/Configurations/BP_UDSWConfig` _returnvalue))
          (bind (_value _returnvalue_2) (`BlueprintMapLibrary.Map_Find` (`/Game/UltraDynamicSky/Blueprints/Configurations/BP_UDSWConfig.UDSWMap` _asbp_udswconfig) Tag))
          (if _returnvalue_2
            (`|ExecutionSequence`
              (:`then_0`
                (bind (_skypreset _weatherpreset _timeofday _skymodifiers _weathersettings) (break `/Game/UltraDynamicSky/Blueprints/Configurations/UDSWConfigEntry` _value))
                (`/Engine/EditorBlueprintResources/StandardMacros.IsValid` (`|ConvertAsset` _skypreset)
                  (:`Is Valid`
                    (`KismetSystemLibrary.PrintString` (`KismetSystemLibrary.GetDisplayName` (`self.UDS`)) true true (struct :`R` 1.0 :`G` 0.072683 :`B` 0.092578 :`A` 1.0) 20.0)
                    (`/Game/UltraDynamicSky/Blueprints/Ultra_Dynamic_Sky.MultiSetSkyPreset` (`self.UDS`) _skypreset))))
              (:`then_1`
                (`/Engine/EditorBlueprintResources/StandardMacros.IsValid` (`|ConvertAsset` _weatherpreset)
                  (:`Is Valid`
                    (`/Game/UltraDynamicSky/Blueprints/Ultra_Dynamic_Weather.MultiSetWeatherPreset` (`self.UDW`) _weatherpreset))))
              (:`then_2`
                (if (>= (break `/Game/UltraDynamicSky/Blueprints/Configurations/UDSTODTransition` _timeofday) 0.0)
                  (if (`self.bFirstStateInited`)
                    (`/Game/UltraDynamicSky/Blueprints/Ultra_Dynamic_Sky.Transition Time of Day` _uds (break `/Game/UltraDynamicSky/Blueprints/Configurations/UDSTODTransition` _timeofday) (`.TransitionTime_5_223E95424463A629B8CFDFB6FF96C248` (break `/Game/UltraDynamicSky/Blueprints/Configurations/UDSTODTransition` _timeofday)) "EaseInOut" 2.0 false)
                    (else
                      (set `self.bFirstStateInited` true)
                      (`/Game/UltraDynamicSky/Blueprints/Ultra_Dynamic_Sky.Transition Time of Day` _uds (break `/Game/UltraDynamicSky/Blueprints/Configurations/UDSTODTransition` _timeofday) 0.0 "EaseInOut" 2.0 true)))))
              (:`then_3`
                (if (`KismetArrayLibrary.Array_IsNotEmpty` _lastudsmodifiers)
                  (for _array_element _lastudsmodifiers
                    (`/Game/UltraDynamicSky/Blueprints/Ultra_Dynamic_Sky.MultiRemoveUDSModifiers` (`self.UDS`) _array_element 10.0)
                    (`KismetArrayLibrary.Array_RemoveItem` (`self.LastUDSModifiers`) _array_element)))
                (for _array_element_2 _skymodifiers
                  (`/Game/UltraDynamicSky/Blueprints/Ultra_Dynamic_Sky.MultiUseUDSModifiers` (`self.UDS`) (break `/Game/UltraDynamicSky/Blueprints/Configurations/UDSModifierTransition` _array_element_2) (`.TransitionTime_5_223E95424463A629B8CFDFB6FF96C248` (break `/Game/UltraDynamicSky/Blueprints/Configurations/UDSModifierTransition` _array_element_2)))
                  (`KismetArrayLibrary.Array_Add` (`self.LastUDSModifiers`) (break `/Game/UltraDynamicSky/Blueprints/Configurations/UDSModifierTransition` _array_element_2))))
              (:`then_4`
                (`/Engine/EditorBlueprintResources/StandardMacros.IsValid` (break `/Game/UltraDynamicSky/Blueprints/Configurations/UDWSettingsTransition` _weathersettings)
                  (:`Is Valid`
                    (`/Game/UltraDynamicSky/Blueprints/Ultra_Dynamic_Weather.Change Weather` (`self.UDW`) (break `/Game/UltraDynamicSky/Blueprints/Configurations/UDWSettingsTransition` _weathersettings) (`.TransitionTime_6_420E39F748DFC763A0C9A18C7F88FF0E` (break `/Game/UltraDynamicSky/Blueprints/Configurations/UDWSettingsTransition` _weathersettings)))))))))
        (:`else`)))
    (:`else`)))

(fn `SetPropertyByName`
  (params (Actor :type "Actor Object Reference") (PropertyName :type Name) (Preset :type "/Game/UltraDynamicSky/Blueprints/System/UDS_Configuration Object Reference") (PropertyType :type "/Game/UltraDynamicSky/Blueprints/Enum/UDS_PropertyType Enum" :default "NewEnumerator0"))
  (bind (_value _returnvalue) (`BlueprintMapLibrary.Map_Find` (`/Game/UltraDynamicSky/Blueprints/System/UDS_Configuration.Vector Properties` (`local.Preset`)) (`local.PropertyName`)))
  (bind (_value_2 _returnvalue_2) (`BlueprintMapLibrary.Map_Find` (`/Game/UltraDynamicSky/Blueprints/System/UDS_Configuration.Soft Object Properties` (`local.Preset`)) (`local.PropertyName`)))
  (bind (_value_3 _returnvalue_3) (`BlueprintMapLibrary.Map_Find` (`/Game/UltraDynamicSky/Blueprints/System/UDS_Configuration.Byte Properties` (`local.Preset`)) (`local.PropertyName`)))
  (bind (_value_4 _returnvalue_4) (`BlueprintMapLibrary.Map_Find` (`/Game/UltraDynamicSky/Blueprints/System/UDS_Configuration.Vector 2D Properties` (`local.Preset`)) (`local.PropertyName`)))
  (bind (_value_5 _returnvalue_5) (`BlueprintMapLibrary.Map_Find` (`/Game/UltraDynamicSky/Blueprints/System/UDS_Configuration.Float Properties` (`local.Preset`)) (`local.PropertyName`)))
  (bind (_value_6 _returnvalue_6) (`BlueprintMapLibrary.Map_Find` (`/Game/UltraDynamicSky/Blueprints/System/UDS_Configuration.Float Range Properties` (`local.Preset`)) (`local.PropertyName`)))
  (bind (_value_7 _returnvalue_7) (`BlueprintMapLibrary.Map_Find` (`/Game/UltraDynamicSky/Blueprints/System/UDS_Configuration.Int Properties` (`local.Preset`)) (`local.PropertyName`)))
  (bind (_value_8 _returnvalue_8) (`BlueprintMapLibrary.Map_Find` (`/Game/UltraDynamicSky/Blueprints/System/UDS_Configuration.Color Properties` (`local.Preset`)) (`local.PropertyName`)))
  (bind (_value_9 _returnvalue_9) (`BlueprintMapLibrary.Map_Find` (`/Game/UltraDynamicSky/Blueprints/System/UDS_Configuration.Object Properties` (`local.Preset`)) (`local.PropertyName`)))
  (bind (_value_10 _returnvalue_10) (`BlueprintMapLibrary.Map_Find` (`/Game/UltraDynamicSky/Blueprints/System/UDS_Configuration.Bool Properties` (`local.Preset`)) (`local.PropertyName`)))
  (switch `/Game/UltraDynamicSky/Blueprints/Enum/UDS_PropertyType` PropertyType
    (:`NewEnumerator0`
      (if _returnvalue_5
        (`KismetSystemLibrary.SetDoublePropertyByName` (`local.Actor`) (`local.PropertyName`) _value_5)))
    (:`NewEnumerator1`
      (if _returnvalue_7
        (`KismetSystemLibrary.SetIntPropertyByName` (`local.Actor`) (`local.PropertyName`) _value_7)))
    (:`NewEnumerator2`
      (if _returnvalue_8
        (`KismetSystemLibrary.SetLinearColorPropertyByName` (`local.Actor`) (`local.PropertyName`) _value_8)))
    (:`NewEnumerator3`
      (if _returnvalue_9
        (`KismetSystemLibrary.SetObjectPropertyByName` (`local.Actor`) (`local.PropertyName`) _value_9)))
    (:`NewEnumerator4`
      (if _returnvalue_10
        (`KismetSystemLibrary.SetBoolPropertyByName` (`local.Actor`) (`local.PropertyName`) _value_10)))
    (:`NewEnumerator5`
      (if _returnvalue_3
        (`KismetSystemLibrary.SetBytePropertyByName` (`local.Actor`) (`local.PropertyName`) _value_3)))
    (:`NewEnumerator6`
      (if _returnvalue_4
        (`KismetSystemLibrary.SetStructurePropertyByName` (`local.Actor`) (`local.PropertyName`) _value_4)))
    (:`NewEnumerator11`
      (if _returnvalue
        (`KismetSystemLibrary.SetVector3fPropertyByName` (`local.Actor`) (`local.PropertyName`) _value)))
    (:`NewEnumerator13`
      (if _returnvalue_2
        (`KismetSystemLibrary.SetSoftObjectPropertyByName` (`local.Actor`) (`local.PropertyName`) _value_2)))
    (:`NewEnumerator14`
      (if _returnvalue_6
        (`KismetSystemLibrary.SetStructurePropertyByName` (`local.Actor`) (`local.PropertyName`) _value_6)))))

(fn `SetUDS`
  (params (ExternalUDS :type "/Game/UltraDynamicSky/Blueprints/Ultra_Dynamic_Sky Object Reference"))
  (bind _output_get (set `self.UDS` ExternalUDS))
  (set `self.UDSToCpp` _output_get)
  (`KismetSystemLibrary.PrintString` "manager set UDS!"))

(fn `SetUDSPreset`
  (params (Preset :type "/Game/UltraDynamicSky/Blueprints/System/UDS_Configuration Object Reference"))
  (locals (`Weather BP Present` :type Boolean) (`Current Property` :type Name) (`Properties Overwritten by Weather` :type "Array of Name"))
  (set `/Game/UltraDynamicSky/Blueprints/Ultra_Dynamic_Sky.Sky Mode Scalability Map` (`/Game/UltraDynamicSky/Blueprints/System/UDS_Configuration.Sky Mode Map` (`local.Preset`)) (`self.UDS`))
  (set `/Game/UltraDynamicSky/Blueprints/Ultra_Dynamic_Sky.Platform Feature Levels` (`/Game/UltraDynamicSky/Blueprints/System/UDS_Configuration.Platform Feature Levels` (`local.Preset`)) (`self.UDS`))
  (set `/Game/UltraDynamicSky/Blueprints/Ultra_Dynamic_Sky.Post Process Components` (`/Game/UltraDynamicSky/Blueprints/System/UDS_Configuration.Post Process Components` (`local.Preset`)) (`self.UDS`))
  (set `/Game/UltraDynamicSky/Blueprints/Ultra_Dynamic_Sky.Static Post Process Settings` (`/Game/UltraDynamicSky/Blueprints/System/UDS_Configuration.Static Post Process Settings` (`local.Preset`)) (`self.UDS`))
  (set `/Game/UltraDynamicSky/Blueprints/Ultra_Dynamic_Sky.Planets/Moons` (`/Game/UltraDynamicSky/Blueprints/System/UDS_Configuration.Planets/Moons` (`local.Preset`)) (`self.UDS`))
  (set `/Game/UltraDynamicSky/Blueprints/Ultra_Dynamic_Sky.Starting Modifiers` (`/Game/UltraDynamicSky/Blueprints/System/UDS_Configuration.Starting Modifiers` (`local.Preset`)) (`self.UDS`))
  (set `local.Weather BP Present` (`KismetSystemLibrary.IsValid` (`self.UDW`)))
  (bind _keys (`BlueprintMapLibrary.Map_Keys` (`/Game/UltraDynamicSky/Blueprints/Ultra_Dynamic_Sky.Properties` (`self.UDS`))))
  (for _array_element _keys
    (set `local.Current Property` _array_element)
    (if (not (and (`local.Weather BP Present`) (`KismetArrayLibrary.Array_Contains` (`local.Properties Overwritten by Weather`) (`local.Current Property`))))
      (`self.SetPropertyByName` (`self.UDS`) (`local.Current Property`) (`local.Preset`) (`BlueprintMapLibrary.Map_Find` (`/Game/UltraDynamicSky/Blueprints/Ultra_Dynamic_Sky.Properties` (`self.UDS`)) (`local.Current Property`))))))

(fn `SetUDW`
  (params (ExternalUDW :type "/Game/UltraDynamicSky/Blueprints/Ultra_Dynamic_Weather Object Reference"))
  (bind _output_get (set `self.UDW` ExternalUDW))
  (set `self.UDWToCpp` _output_get)
  (`KismetSystemLibrary.PrintString` "manager set UDW!"))

(fn `SetUDWPreset`
  (params (Preset :type "/Game/UltraDynamicSky/Blueprints/System/UDS_Configuration Object Reference"))
  (bind _keys (`BlueprintMapLibrary.Map_Keys` (`/Game/UltraDynamicSky/Blueprints/Ultra_Dynamic_Weather.Properties` (`self.UDW`))))
  (for _array_element _keys
    (`self.SetPropertyByName` (`self.UDW`) _array_element (`local.Preset`) (`BlueprintMapLibrary.Map_Find` (`/Game/UltraDynamicSky/Blueprints/Ultra_Dynamic_Weather.Properties` (`self.UDW`)) _array_element)))
  (`|ExecutionSequence`
    (:`then_0`
      (set `/Game/UltraDynamicSky/Blueprints/Ultra_Dynamic_Weather.Weather Type Probabilities (Autumn)` (`/Game/UltraDynamicSky/Blueprints/System/UDS_Configuration.Weather Probability (Autumn)` (`local.Preset`)) (`self.UDW`))
      (set `/Game/UltraDynamicSky/Blueprints/Ultra_Dynamic_Weather.Weather Type Probabilities (Spring)` (`/Game/UltraDynamicSky/Blueprints/System/UDS_Configuration.Weather Probability (Spring)` (`local.Preset`)) (`self.UDW`))
      (set `/Game/UltraDynamicSky/Blueprints/Ultra_Dynamic_Weather.Weather Type Probabilities (Summer)` (`/Game/UltraDynamicSky/Blueprints/System/UDS_Configuration.Weather Probability (Summer)` (`local.Preset`)) (`self.UDW`))
      (set `/Game/UltraDynamicSky/Blueprints/Ultra_Dynamic_Weather.Weather Type Probabilities (Winter)` (`/Game/UltraDynamicSky/Blueprints/System/UDS_Configuration.Weather Probability (Winter)` (`local.Preset`)) (`self.UDW`))
      (set `/Game/UltraDynamicSky/Blueprints/Ultra_Dynamic_Weather.Weather Specific Interval Multipliers` (`/Game/UltraDynamicSky/Blueprints/System/UDS_Configuration.Weather Specific Interval Multipliers` (`local.Preset`)) (`self.UDW`))
      (set `/Game/UltraDynamicSky/Blueprints/Ultra_Dynamic_Weather.Physical Materials which disable Puddle Sounds and Particles` (`/Game/UltraDynamicSky/Blueprints/System/UDS_Configuration.PhysMats_Disable Puddles` (`local.Preset`)) (`self.UDW`))
      (set `/Game/UltraDynamicSky/Blueprints/Ultra_Dynamic_Weather.Physical Materials which disable Snow/Dust Sounds and Particles` (`/Game/UltraDynamicSky/Blueprints/System/UDS_Configuration.PhysMats_Disable Snow` (`local.Preset`)) (`self.UDW`)))
    (:`then_1`
      (`/Game/UltraDynamicSky/Blueprints/Ultra_Dynamic_Weather.Construction Script Function` (`self.UDW`)))))

(fn `UDSIsValid`
  (returns (ReturnValue :type Boolean))
  (`self.UDS`
    (:`then`
      (return true))
    (:`else`
      (return false))))

(fn `UDWIsValid`
  (returns (ReturnValue :type Boolean))
  (`self.UDW`
    (:`then`
      (return true))
    (:`else`
      (return false))))